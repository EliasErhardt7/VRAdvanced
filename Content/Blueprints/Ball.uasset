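; Ball is an actor that applies its own downward gravity to its Ball component once it has been thrown.
; On BeginPlay it enables input from player controller 0.
; Each tick while IsThrow is set, it adds a downward force equal to GravityStrength times the ball's mass, giving a tunable, mass-independent fall acceleration.
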(event EventBeginPlay
  (Input|EnableInput (Game|GetPlayerController 0)))

(event Collision|EventActorBeginOverlap
  (params (OtherActor :type Actor%20Object%20Reference)))

(event EventTick
  (params (DeltaSeconds :type Float%20%28single-precision%29))
  (if (Variables|Default|GetisThrow)
    (Physics|AddForce (Variables|Default|GetBall) (* (* (Variables|Default|GetgravityStrength) (Physics|GetMass (Variables|Default|GetBall))) "0.000000,0.000000,-1.000000") "None" false)))

(fn ConstructionScript)