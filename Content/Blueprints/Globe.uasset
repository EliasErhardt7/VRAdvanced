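; Globe actor that displays a spinning sphere which the player can switch between celestial bodies.
; BeginPlay enables input from player controller 0, and input actions swap the sphere's material to Earth, Moon, Sun, Jupiter, Pluto or Mars.
; Tick adds a fixed world rotation to the sphere every frame, so spin speed depends on frame rate rather than delta time.
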(event Input|EnhancedActionEvents|EnhancedInputActionJupiterButton
  (params (ActionValue :type Boolean) (ElapsedSeconds :type Float%20%28double-precision%29) (TriggeredSeconds :type Float%20%28double-precision%29) (InputAction :type Input%20Action%20Object%20Reference :default "/Game/Blueprints/JupiterButton.JupiterButton"))
  ;[0.15 0.15 0.15 0.5] Jupiter
  (Rendering|Material|SetMaterial (Variables|Default|GetSphere) 0 "/Game/Environment/Jupiter.Jupiter"))

(event Input|EnhancedActionEvents|EnhancedInputActionSunButton
  (params (ActionValue :type Boolean) (ElapsedSeconds :type Float%20%28double-precision%29) (TriggeredSeconds :type Float%20%28double-precision%29) (InputAction :type Input%20Action%20Object%20Reference :default "/Game/Blueprints/SunButton.SunButton"))
  ;[0.15 0.15 0.15 0.5] Sun
  (Rendering|Material|SetMaterial (Variables|Default|GetSphere) 0 "/Game/Environment/Sun.Sun"))

(event Input|EnhancedActionEvents|EnhancedInputActionMarsButton
  (params (ActionValue :type Boolean) (ElapsedSeconds :type Float%20%28double-precision%29) (TriggeredSeconds :type Float%20%28double-precision%29) (InputAction :type Input%20Action%20Object%20Reference :default "/Game/Blueprints/MarsButton.MarsButton"))
  ;[0.15 0.15 0.15 0.5] Mars
  (Rendering|Material|SetMaterial (Variables|Default|GetSphere) 0 "/Game/Environment/Mars.Mars"))

(event Input|EnhancedActionEvents|EnhancedInputActionPlutoButton
  (params (ActionValue :type Boolean) (ElapsedSeconds :type Float%20%28double-precision%29) (TriggeredSeconds :type Float%20%28double-precision%29) (InputAction :type Input%20Action%20Object%20Reference :default "/Game/Blueprints/PlutoButton.PlutoButton"))
  ;[0.15 0.15 0.15 0.5] Sun
  (Rendering|Material|SetMaterial (Variables|Default|GetSphere) 0 "/Game/Environment/Pluto.Pluto"))

(event Input|EnhancedActionEvents|EnhancedInputActionEarthButton
  (params (ActionValue :type Boolean) (ElapsedSeconds :type Float%20%28double-precision%29) (TriggeredSeconds :type Float%20%28double-precision%29) (InputAction :type Input%20Action%20Object%20Reference :default "/Game/Blueprints/EarthButton.EarthButton"))
  ;[0.15 0.15 0.15 0.5] Earth
  (Rendering|Material|SetMaterial (Variables|Default|GetSphere) 0 "/Game/Environment/Earth.Earth"))

(event Input|EnhancedActionEvents|EnhancedInputActionMoonButton
  (params (ActionValue :type Boolean) (ElapsedSeconds :type Float%20%28double-precision%29) (TriggeredSeconds :type Float%20%28double-precision%29) (InputAction :type Input%20Action%20Object%20Reference :default "/Game/Blueprints/MoonButton.MoonButton"))
  ;[0.15 0.15 0.15 0.5] Moon
  (Rendering|Material|SetMaterial (Variables|Default|GetSphere) 0 "/Game/Environment/Moon.Moon"))

(event EventBeginPlay
  (Input|EnableInput (Game|GetPlayerController 0)))

(event Collision|EventActorBeginOverlap
  (params (OtherActor :type Actor%20Object%20Reference)))

(event EventTick
  (params (DeltaSeconds :type Float%20%28single-precision%29))
  (Transformation|AddWorldRotation (Variables|Default|GetSphere) "0.000000,1.000000,0.000000" false false))

(fn ConstructionScript)