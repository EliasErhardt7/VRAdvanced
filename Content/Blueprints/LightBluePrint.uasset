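; Light controller Blueprint that switches a directional light between presets themed on celestial bodies: Earth, Sun, Moon, Mars, Jupiter and Pluto.
; On BeginPlay it enables input from the first player controller and applies a default pale blue tint to DirectionalLight1.
; Each body's input action directly sets a hardcoded color and intensity on that light, with no blending or stored state.
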(event Input|EnhancedActionEvents|EnhancedInputActionJupiterButton
  (params (ActionValue :type Boolean) (ElapsedSeconds :type Float%20%28double-precision%29) (TriggeredSeconds :type Float%20%28double-precision%29) (InputAction :type Input%20Action%20Object%20Reference :default "/Game/Blueprints/JupiterButton.JupiterButton"))
  (bind _directionallight1 (Variables|Default|GetDirectionalLight1))
  ;[0.15 0.15 0.15 0.5] Jupiter
  (Rendering|Components|Light|SetLightColor _directionallight1 "(R=1.000000,G=0.340492,B=0.093750,A=1.000000)" true)
  (Rendering|Components|Light|SetIntensity _directionallight1 14.0))

(event Input|EnhancedActionEvents|EnhancedInputActionSunButton
  (params (ActionValue :type Boolean) (ElapsedSeconds :type Float%20%28double-precision%29) (TriggeredSeconds :type Float%20%28double-precision%29) (InputAction :type Input%20Action%20Object%20Reference :default "/Game/Blueprints/SunButton.SunButton"))
  (bind _directionallight1 (Variables|Default|GetDirectionalLight1))
  ;[0.15 0.15 0.15 0.5] Sun
  (Rendering|Components|Light|SetLightColor _directionallight1 "(R=1.000000,G=0.253414,B=0.022275,A=1.000000)" true)
  (Rendering|Components|Light|SetIntensity _directionallight1 5e+01))

(event Input|EnhancedActionEvents|EnhancedInputActionMarsButton
  (params (ActionValue :type Boolean) (ElapsedSeconds :type Float%20%28double-precision%29) (TriggeredSeconds :type Float%20%28double-precision%29) (InputAction :type Input%20Action%20Object%20Reference :default "/Game/Blueprints/MarsButton.MarsButton"))
  (bind _directionallight1 (Variables|Default|GetDirectionalLight1))
  ;[0.15 0.15 0.15 0.5] Mars
  (Rendering|Components|Light|SetLightColor _directionallight1 "(R=1.000000,G=0.009645,B=0.000000,A=1.000000)" true)
  (Rendering|Components|Light|SetIntensity _directionallight1 7.0))

(event Input|EnhancedActionEvents|EnhancedInputActionPlutoButton
  (params (ActionValue :type Boolean) (ElapsedSeconds :type Float%20%28double-precision%29) (TriggeredSeconds :type Float%20%28double-precision%29) (InputAction :type Input%20Action%20Object%20Reference :default "/Game/Blueprints/PlutoButton.PlutoButton"))
  (bind _directionallight1 (Variables|Default|GetDirectionalLight1))
  ;[0.15 0.15 0.15 0.5] Pluto
  (Rendering|Components|Light|SetLightColor _directionallight1 "(R=0.104957,G=0.000000,B=1.000000,A=1.000000)" true)
  (Rendering|Components|Light|SetIntensity _directionallight1 6.0))

(event Input|EnhancedActionEvents|EnhancedInputActionEarthButton
  (params (ActionValue :type Boolean) (ElapsedSeconds :type Float%20%28double-precision%29) (TriggeredSeconds :type Float%20%28double-precision%29) (InputAction :type Input%20Action%20Object%20Reference :default "/Game/Blueprints/EarthButton.EarthButton"))
  (bind _directionallight1 (Variables|Default|GetDirectionalLight1))
  ;[0.15 0.15 0.15 0.5] Earth
  (Rendering|Components|Light|SetLightColor _directionallight1 "(R=0.703903,G=1.000000,B=0.806109,A=1.000000)" true)
  (Rendering|Components|Light|SetIntensity _directionallight1 1e+01))

(event Input|EnhancedActionEvents|EnhancedInputActionMoonButton
  (params (ActionValue :type Boolean) (ElapsedSeconds :type Float%20%28double-precision%29) (TriggeredSeconds :type Float%20%28double-precision%29) (InputAction :type Input%20Action%20Object%20Reference :default "/Game/Blueprints/MoonButton.MoonButton"))
  (bind _directionallight1 (Variables|Default|GetDirectionalLight1))
  ;[0.15 0.15 0.15 0.5] Moon
  (Rendering|Components|Light|SetLightColor _directionallight1 "(R=0.640210,G=0.867421,B=1.000000,A=1.000000)" true)
  (Rendering|Components|Light|SetIntensity _directionallight1 16.0))

(event EventBeginPlay
  (bind _directionallight1 (Variables|Default|GetDirectionalLight1))
  (Input|EnableInput (Game|GetPlayerController 0))
  (Rendering|Components|Light|SetLightColor _directionallight1 "(R=0.520996,G=0.590619,B=1.000000,A=1.000000)" true)
  (Rendering|Components|Light|SetIntensity _directionallight1 1e+01))

(event Collision|EventActorBeginOverlap
  (params (OtherActor :type Actor%20Object%20Reference)))

(event EventTick
  (params (DeltaSeconds :type Float%20%28single-precision%29)))

(fn ConstructionScript)