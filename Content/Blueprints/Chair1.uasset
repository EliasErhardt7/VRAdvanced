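; Chair1 is a target actor that reacts when a Ball overlaps its Box, acting as a scoring hit.
; On a hit it spawns a replacement Chair1 at a randomized offset from a fixed world point with random roll, plays a score sound, then destroys itself.
; When a Ball's overlap with the Box ends, that Ball is destroyed.
; It also enables input from the first player controller on BeginPlay.
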(event OnComponentEndOverlap(Box)
  (params (OverlappedComponent :type Primitive%20Component%20Object%20Reference) (OtherActor :type Actor%20Object%20Reference) (OtherComp :type Primitive%20Component%20Object%20Reference) (OtherBodyIndex :type Integer))
  (bind _asball (Utilities|Casting|CastToBall OtherActor))
  (Actor|DestroyActor _asball))

(event OnComponentBeginOverlap(Box)
  (params (OverlappedComponent :type Primitive%20Component%20Object%20Reference) (OtherActor :type Actor%20Object%20Reference) (OtherComp :type Primitive%20Component%20Object%20Reference) (OtherBodyIndex :type Integer) (bFromSweep :type Boolean) (SweepResult :type Hit%20Result%20Structure%20%28by%20ref%29))
  (bind _box (Variables|Default|GetBox))
  (bind _returnvalue (Transformation|GetWorldRotation _box))
  (Utilities|Casting|CastToBall OtherActor)
  (Game|SpawnActorfromClass "Chair1_C" (Math|Transform|MakeTransform (+ "-47.000000,-900.000000,174.000000" (Math|Vector|MakeVector (Math|Conversions|ToFloat(Integer) (Math|Random|RandomIntegerinRange -300 300)) (Math|Conversions|ToFloat(Integer) (Math|Random|RandomIntegerinRange 0 300)) (Math|Conversions|ToFloat(Integer) (Math|Random|RandomIntegerinRange -100 100)))) (Math|Rotator|MakeRotator (+ (.roll _returnvalue) (Math|Random|RandomFloatinRange 0.0 3.6e+02)) (.pitch _returnvalue) (.yaw _returnvalue)) "1.000000,1.000000,1.000000") "Undefined" "MultiplyWithRoot" 0 0 0)
  (Audio|PlaySoundatLocation "/Game/Blueprints/ScoreSound.ScoreSound" (Transformation|GetWorldLocation (Variables|Default|GetHalfCircle)) "0, 0, 0" 1.0 1.0 0.0 0 0 0 0)
  (Actor|DestroyActor))

(event EventBeginPlay
  (Input|EnableInput (Game|GetPlayerController 0)))

(event Collision|EventActorBeginOverlap
  (params (OtherActor :type Actor%20Object%20Reference)))

(event EventTick
  (params (DeltaSeconds :type Float%20%28single-precision%29)))

(fn ConstructionScript)