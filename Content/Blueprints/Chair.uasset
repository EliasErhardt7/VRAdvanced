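; Chair actor that shows a widget while the player character stands inside its box trigger.
; BeginPlay caches the player character as a TestCharacter.
; The Box begin and end overlap events compare the overlapping actor to that cached reference, then set the Widget visible or hidden.
; The file contains no sitting or other interaction logic.
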(event OnComponentEndOverlap(Box)
  (params (OverlappedComponent :type Primitive%20Component%20Object%20Reference) (OtherActor :type Actor%20Object%20Reference) (OtherComp :type Primitive%20Component%20Object%20Reference) (OtherBodyIndex :type Integer))
  (if (== OtherActor (Variables|Default|GetAs%20Test%20Character))
    (Rendering|SetVisibility (Variables|Default|GetWidget) false false)))

(event OnComponentBeginOverlap(Box)
  (params (OverlappedComponent :type Primitive%20Component%20Object%20Reference) (OtherActor :type Actor%20Object%20Reference) (OtherComp :type Primitive%20Component%20Object%20Reference) (OtherBodyIndex :type Integer) (bFromSweep :type Boolean) (SweepResult :type Hit%20Result%20Structure%20%28by%20ref%29))
  (if (== OtherActor (Variables|Default|GetAs%20Test%20Character))
    (Rendering|SetVisibility (Variables|Default|GetWidget) true false)))

(event EventBeginPlay
  (bind _astest_character (Utilities|Casting|CastToTestCharacter (Game|GetPlayerCharacter 0)))
  (Variables|Default|SetAs%20Test%20Character _astest_character))

(event Collision|EventActorBeginOverlap
  (params (OtherActor :type Actor%20Object%20Reference)))

(event EventTick
  (params (DeltaSeconds :type Float%20%28single-precision%29)))

(fn ConstructionScript)